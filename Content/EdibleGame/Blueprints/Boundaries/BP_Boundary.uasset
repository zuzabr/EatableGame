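; Play-field actor for an edible/inedible sorting game that spawns objects and judges which boundary they reach.
; After GS_Edible supplies object data and signals game start, a looping timer, pausable by events, spawns random BP_SpawnObjDafault items at five points.
; Left and right overlaps compare edibility against EdibleOnTheLeft, while the bottom means a loss.
; Outcomes are only printed, and each overlapping object is passed to BP_PlController's StopCarryDestroyedObject.
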(event OnComponentBeginOverlap(BoundaryLeft)
  (params (OverlappedComponent :type Primitive%20Component%20Object%20Reference) (OtherActor :type Actor%20Object%20Reference) (OtherComp :type Primitive%20Component%20Object%20Reference) (OtherBodyIndex :type Integer) (bFromSweep :type Boolean) (SweepResult :type Hit%20Result%20Structure%20%28by%20ref%29))
  ;[1 1 1] Пересечение с границами
  (bind _asbp_spawn_obj_dafault (Utilities|Casting|CastToBP_SpawnObjDafault OtherActor))
  (if (Variables|Default|GetEdibleOnTheLeft)
    (if (Default|GetEdible _asbp_spawn_obj_dafault)
      (Development|PrintString "You Are Right!")
      (else
        (Development|PrintString "You Are Wrong!")))
    (elif (Default|GetEdible _asbp_spawn_obj_dafault)
      (Development|PrintString "You Are Wrong!")
      (else
        (Development|PrintString "You Are Right!"))))
  (bind _asbp_pl_controller (Utilities|Casting|CastToBP_PlController (Game|GetPlayerController 0)))
  (Default|StopCarryDestroyedObject _asbp_pl_controller _asbp_spawn_obj_dafault))

(event OnComponentBeginOverlap(BoundaryRight)
  (params (OverlappedComponent :type Primitive%20Component%20Object%20Reference) (OtherActor :type Actor%20Object%20Reference) (OtherComp :type Primitive%20Component%20Object%20Reference) (OtherBodyIndex :type Integer) (bFromSweep :type Boolean) (SweepResult :type Hit%20Result%20Structure%20%28by%20ref%29))
  ;[1 1 1] Пересечение с границами
  (bind _asbp_spawn_obj_dafault (Utilities|Casting|CastToBP_SpawnObjDafault OtherActor))
  (if (Variables|Default|GetEdibleOnTheLeft)
    (if (Default|GetEdible _asbp_spawn_obj_dafault)
      (Development|PrintString "You Are Wrong!")
      (else
        (Development|PrintString "You Are Right!")))
    (elif (Default|GetEdible _asbp_spawn_obj_dafault)
      (Development|PrintString "You Are Right!")
      (else
        (Development|PrintString "You Are Wrong!"))))
  (bind _asbp_pl_controller (Utilities|Casting|CastToBP_PlController (Game|GetPlayerController 0)))
  (Default|StopCarryDestroyedObject _asbp_pl_controller _asbp_spawn_obj_dafault))

(event OnComponentBeginOverlap(BoundaryBottom)
  (params (OverlappedComponent :type Primitive%20Component%20Object%20Reference) (OtherActor :type Actor%20Object%20Reference) (OtherComp :type Primitive%20Component%20Object%20Reference) (OtherBodyIndex :type Integer) (bFromSweep :type Boolean) (SweepResult :type Hit%20Result%20Structure%20%28by%20ref%29))
  ;[1 1 1] Пересечение с границами
  (bind _asbp_spawn_obj_dafault (Utilities|Casting|CastToBP_SpawnObjDafault OtherActor))
  (Development|PrintString "You Lose!")
  (bind _asbp_pl_controller (Utilities|Casting|CastToBP_PlController (Game|GetPlayerController 0)))
  (Default|StopCarryDestroyedObject _asbp_pl_controller _asbp_spawn_obj_dafault))

(event Custom|Start%20Game%20Session
  (Utilities|Time|UnpauseTimerbyHandle (Variables|Timer|GetSpawnTimer)))

(event Custom|End%20Game%20Session
  ;[1 1 1] Начало/Пауза/Остановка игровой сессии
  (Utilities|Time|PauseTimerbyHandle (Variables|Timer|GetSpawnTimer)))

(event Custom|PauseTheGame
  ;[1 1 1] Начало/Пауза/Остановка игровой сессии
  (Utilities|Time|PauseTimerbyHandle (Variables|Timer|GetSpawnTimer)))

(event EventBeginPlay
  (Utilities|FlowControl|Delay 0.2)
  (CallFunction|SetSpawnObjInfo)
  (EventDispatchers|BindEventtoStartGame (Variables|Default|GetGameState) (delegate Custom|Start%20Game%20Session))
  (bind _returnvalue (Utilities|Time|SetTimerbyFunctionName 0 "SpawnObjects" (Variables|Timer|GetTime) true))
  (bind _output_get (Variables|Timer|SetSpawnTimer _returnvalue))
  (Utilities|Time|PauseTimerbyHandle _output_get))

(fn ConstructionScript
  (Rendering|Components|Sprite|SetSprite (Variables|Default|GetPaperSprite) "/Game/EdibleGame/Sprites/BackGround/PS_Farm.PS_Farm"))

(fn SpawnObjects
  (bind _objtospawn (CallFunction|PickObjtoSpawn))
  (Game|SpawnActorfromClass "/Game/EdibleGame/Blueprints/Core/BP_SpawnObjDafault.BP_SpawnObjDafault_C" (Math|Transform|MakeTransform (Transformation|GetWorldLocation (Utilities|Select :Index (Math|Random|RandomIntegerinRange 0 4) :Option%200 (Variables|Default|GetSpawnPoint1) :Option%201 (Variables|Default|GetSpawnPoint2) :Option%202 (Variables|Default|GetSpawnPoint3) :Option%203 (Variables|Default|GetSpawnPoint4) :Option%204 (Variables|Default|GetSpawnPoint5))) "0, 0, 0" "1.000000,1.000000,1.000000") "AdjustIfPossibleButAlwaysSpawn" 0 _objtospawn 0))

(fn PickObjtoSpawn
  (return (Utilities|Array|Get(acopy) (Variables|Default|GetSpawn%20Obj%20Info) (Math|Random|RandomIntegerinRange 0 (- (Utilities|Array|Length (Variables|Default|GetSpawn%20Obj%20Info)) 1)))))

(fn SetSpawnObjInfo
  (bind _asgs_edible (Utilities|Casting|CastToGS_Edible (Game|GetGameState)))
  (Variables|Default|SetGameState _asgs_edible)
  (Variables|Default|SetSpawn%20Obj%20Info (Default|GetSpawnObjInfo (Variables|Default|GetGameState))))