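; Player controller that lets the player drag physics-simulated BP_SpawnObjDafault actors with multiple fingers at once.
; Touch press traces under the finger, grabs the hit component with that actor's own PhysicsHandle, and records it by finger index in GrabbedObjects.
; Touch move updates the handle target in X and Z, keeping the object's Y, and touch release drops it.
; StopCarryDestroyedObject releases a held object before destroying it.
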(event Custom|StopCarryDestroyedObject
  (params (CarriedObject :type BP%20Spawn%20Obj%20Dafault%20Object%20Reference))
  (Carry|DestroyActor CarriedObject))

(event EventBeginPlay)

(event Input|TouchEvents|InputTouch
  (params (Location :type Vector) (FingerIndex :type ETouchIndex%20Enum))
  (:Pressed
    (Carry|StartCarry FingerIndex))
  (:Released
    (Carry|StopCarry FingerIndex))
  (:Moved
    (Carry|UpdateCarry FingerIndex)))

(fn ConstructionScript)

(fn StartCarry
  (params (FingerIndex :type ETouchIndex%20Enum :default "Touch1"))
  (bind _output_get (LocalVariables|SetL_FingerIndex FingerIndex))
  (bind _alreadycarry (Support|CheckforCarry _output_get))
  (if (not _alreadycarry)
    (bind _asbp_spawn_obj_dafault (Utilities|Casting|CastToBP_SpawnObjDafault (.HitActor (Collision|BreakHitResult (.HitResult (Class|PlayerController|GetHitResultUnderFingerbyChannel (LocalVariables|GetL_FingerIndex) "TraceTypeQuery1" true))))))
    (LocalVariables|SetL_CarriedActor _asbp_spawn_obj_dafault)
    (LocalVariables|SetL_HitComp (.HitComponent (Collision|BreakHitResult (.HitResult (Class|PlayerController|GetHitResultUnderFingerbyChannel (LocalVariables|GetL_FingerIndex) "TraceTypeQuery1" true)))))
    (if (Class|SceneComponent|IsAnySimulatingPhysics (.HitComponent (Collision|BreakHitResult (.HitResult (Class|PlayerController|GetHitResultUnderFingerbyChannel (LocalVariables|GetL_FingerIndex) "TraceTypeQuery1" true)))))
      (Class|PhysicsHandleComponent|GrabComponentatLocation (Variables|/Game/EdibleGame/Blueprints/Core/BP_SpawnObjDafault.BP_SpawnObjDafault_C|GetPhysicsHandle (LocalVariables|GetL_CarriedActor)) (LocalVariables|GetL_HitComp) "None" (Transformation|GetWorldLocation (LocalVariables|GetL_HitComp)))
      (Utilities|Array|Add (Variables|Support|GetGrabbedObjects) (Utilities|Struct|MakeST_Grab (LocalVariables|GetL_CarriedActor) (LocalVariables|GetL_HitComp) (LocalVariables|GetL_FingerIndex))))))

(fn StopCarry
  (params (FingerIndex :type ETouchIndex%20Enum :default "Touch1"))
  (bind (_found _index _grab) (Support|CheckforRelease FingerIndex))
  (if _found
    (LocalVariables|SetL_Index _index)
    (Utilities|IsValid (Class|PhysicsHandleComponent|GetGrabbedComponent (Variables|/Game/EdibleGame/Blueprints/Core/BP_SpawnObjDafault.BP_SpawnObjDafault_C|GetPhysicsHandle (.Actor (Utilities|Struct|BreakST_Grab _grab))))
      (:Is%20Valid
        (Physics|Components|PhysicsHandle|ReleaseComponent (Variables|/Game/EdibleGame/Blueprints/Core/BP_SpawnObjDafault.BP_SpawnObjDafault_C|GetPhysicsHandle (.Actor (Utilities|Struct|BreakST_Grab _grab))))
        (Utilities|Array|RemoveIndex (Variables|Support|GetGrabbedObjects) (LocalVariables|GetL_Index))))))

(fn UpdateCarry
  (params (FingerIndex :type ETouchIndex%20Enum :default "Touch1"))
  (bind _hitresult (Class|PlayerController|GetHitResultUnderFingerbyChannel FingerIndex "TraceTypeQuery1" true))
  (bind _location (Collision|BreakHitResult _hitresult))
  (bind (_found _index _grab) (Support|CheckforRelease FingerIndex))
  (if _found
    (Physics|Components|PhysicsHandle|SetTargetLocation (Variables|/Game/EdibleGame/Blueprints/Core/BP_SpawnObjDafault.BP_SpawnObjDafault_C|GetPhysicsHandle (.Actor (Utilities|Struct|BreakST_Grab _grab))) (Math|Vector|MakeVector (.x _location) (.y (Transformation|GetWorldLocation (Class|PhysicsHandleComponent|GetGrabbedComponent (Variables|/Game/EdibleGame/Blueprints/Core/BP_SpawnObjDafault.BP_SpawnObjDafault_C|GetPhysicsHandle (.Actor (Utilities|Struct|BreakST_Grab _grab)))))) (.z _location)))))

(fn CheckforCarry
  (params (Finger%20Index :type ETouchIndex%20Enum :default "Touch1"))
  (LocalVariables|SetL_AlreadyCarry false)
  (if (> (Utilities|Array|Length (Variables|Support|GetGrabbedObjects)) 0)
    (bind _array_element (Utilities|Array|ForEachLoopwithBreak (Variables|Support|GetGrabbedObjects) :!label _label)
      (:LoopBody
        (if (Utilities|Enum|Equal(Enum) (.TouchIndex (Utilities|Struct|BreakST_Grab _array_element)) Finger%20Index)
          (LocalVariables|SetL_AlreadyCarry true)
          (goto _label Break)))
      (:Completed
        (return (LocalVariables|GetL_AlreadyCarry))))
    (else
      (return (LocalVariables|GetL_AlreadyCarry)))))

(fn CheckforRelease
  (params (FingerIndex :type ETouchIndex%20Enum :default "Touch1"))
  (LocalVariables|SetL_ObjFound false)
  (bind (_array_element _array_index) (Utilities|Array|ForEachLoopwithBreak (Variables|Support|GetGrabbedObjects) :!label _label)
    (:LoopBody
      (if (Utilities|Enum|Equal(Enum) (.TouchIndex (Utilities|Struct|BreakST_Grab _array_element)) FingerIndex)
        (LocalVariables|SetL_Index _array_index)
        (LocalVariables|SetL_Grab _array_element)
        (LocalVariables|SetL_ObjFound true)
        (goto _label Break)))
    (:Completed
      (return (LocalVariables|GetL_ObjFound) (LocalVariables|GetL_Index) (LocalVariables|GetL_Grab)))))

(fn CheckforDestroy
  (params (Actor :type BP%20Spawn%20Obj%20Dafault%20Object%20Reference))
  (Utilities|IsValid Actor
    (:Is%20Valid
      (LocalVariables|SetL_Found false)
      (bind (_array_element _array_index) (Utilities|Array|ForEachLoopwithBreak (Variables|Support|GetGrabbedObjects) :!label _label)
        (:LoopBody
          (if (== (.Actor (Utilities|Struct|BreakST_Grab _array_element)) Actor)
            (LocalVariables|SetL_Index _array_index)
            (LocalVariables|SetGrab _array_element)
            (LocalVariables|SetL_Found true)
            (goto _label Break)))
        (:Completed
          (return (LocalVariables|GetL_Found) (LocalVariables|GetL_Index) (LocalVariables|GetGrab)))))
    (:Is%20Not%20Valid
      (return false 0 ""))))

(fn DestroyActor
  (params (CarriedObj :type BP%20Spawn%20Obj%20Dafault%20Object%20Reference))
  (bind (_found _index _grabobj) (Support|CheckforDestroy CarriedObj))
  (if _found
    (Utilities|IsValid (Class|PhysicsHandleComponent|GetGrabbedComponent (Variables|/Game/EdibleGame/Blueprints/Core/BP_SpawnObjDafault.BP_SpawnObjDafault_C|GetPhysicsHandle (.actor _grabobj)))
      (:Is%20Valid
        (if (== (Class|PhysicsHandleComponent|GetGrabbedComponent (Variables|/Game/EdibleGame/Blueprints/Core/BP_SpawnObjDafault.BP_SpawnObjDafault_C|GetPhysicsHandle (.actor _grabobj))) (Variables|/Script/Paper2D.PaperSpriteActor|GetRenderComponent CarriedObj))
          (Carry|StopCarry (.touchindex _grabobj))))
      (:Is%20Not%20Valid
        _)))
  (Actor|DestroyActor CarriedObj))