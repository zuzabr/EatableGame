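; GS_Edible is the game state for the Edible game, handling session UI flow and spawnable object data.
; On BeginPlay it shows the start menu and caches every DT_SpawnObject row into SpawnObjInfo, exposed through a getter.
; StartGameSession fires CallStartGame and shows the main UI.
; A separate function opens the pause widget and pauses the game.
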(event Custom|StartGameSession
  (Default|CallStartGame)
  (Widgets|ShowMainUI))

(event EventBeginPlay
  (Widgets|ShowStartMenu)
  (SpawnObjects|CreateSpawnObjInfo))

(fn ConstructionScript)

(fn CreateSpawnObjInfo
  (bind _outrownames (DataTable|GetDataTableRowNames "/Game/EdibleGame/Blueprints/Core/DT_SpawnObject.DT_SpawnObject"))
  (for _array_element _outrownames
    (bind _returnvalue (Utilities|GetDataTableRow (.DataTable (Utilities|Struct|BreakDataTableRowHandle (Utilities|Struct|MakeDataTableRowHandle "/Game/EdibleGame/Blueprints/Core/DT_SpawnObject.DT_SpawnObject" _array_element))) (.RowName (Utilities|Struct|BreakDataTableRowHandle (Utilities|Struct|MakeDataTableRowHandle "/Game/EdibleGame/Blueprints/Core/DT_SpawnObject.DT_SpawnObject" _array_element))))
      (:then
        (Utilities|Array|Add (Variables|Default|GetSpawnObjInfo) _returnvalue)))))

(fn GetSpawnObjInfo
  (return (Variables|Default|GetSpawnObjInfo)))

(fn ShowStartMenu
  (bind _returnvalue (UserInterface|CreateWidget "/Game/EdibleGame/Widgets/W_StartMenu.W_StartMenu_C" (Game|GetPlayerController 0)))
  (UserInterface|Viewport|AddtoViewport _returnvalue 0))

(fn ShowPauseMenu
  (bind _returnvalue (UserInterface|CreateWidget "/Game/EdibleGame/Widgets/W_Pause.W_Pause_C" (Game|GetPlayerController 0)))
  (UserInterface|Viewport|AddtoViewport _returnvalue 0)
  (Game|SetGamePaused true))

(fn ShowMainUI
  (bind _returnvalue (UserInterface|CreateWidget "/Game/EdibleGame/Widgets/W_MainUI.W_MainUI_C" (Game|GetPlayerController 0)))
  (UserInterface|Viewport|AddtoViewport _returnvalue 0))